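; Base HUD Blueprint that puts the gameplay and shop widgets on screen for the owning player.
; On BeginPlay it creates and adds WBP_GamePlay, then creates ShopRound, stores it as ShopWidget and adds every entry in the MenuWidgets array to the viewport.
; OpenShopWidget and CloseShopWidget events toggle the existing shop widget between visible and collapsed rather than recreating it.
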(event `self.ReceiveBeginPlay`
  ;[1 1 1] Add Game Widget
  (bind _returnvalue (`|CreateWidget` "/Game/Blueprints/Widgets/WBP_GamePlay.WBP_GamePlay_C" (`self.GetOwningPlayerController`)))
  (`UserWidget.AddToViewport` _returnvalue 0)
  ;[1 1 1] Add Shop Widget
  (bind _returnvalue_2 (`|CreateWidget` "/Game/Blueprints/Widgets/ShopRound.ShopRound_C" (`self.GetOwningPlayerController`)))
  (bind _output_get (set `self.ShopWidget` _returnvalue_2))
  (`KismetArrayLibrary.Array_Add` (`self.Menu Widgets`) _output_get)
  (for _array_element (`self.Menu Widgets`)
    (`UserWidget.AddToViewport` _array_element 0)))

(event `OpenShopWidget`
  (set `Widget.Visibility` "Visible" (`self.ShopWidget`)))

(event `CloseShopWidget`
  (`Widget.SetVisibility` (`self.ShopWidget`) "Collapsed"))

(fn `UserConstructionScript`)