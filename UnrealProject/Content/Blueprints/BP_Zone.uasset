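; BP_Zone is an interactable area, blocked by a cube until opened, available when game state currency covers its OpenPrice.
; Interact calls a server RPC that sets the open state, relays it through RPC_openZone and notifies BP_GameState.
; SetZoneState hides the cube and switches its collision between BlockAll and OverlapAll.
; Shopper enter/exit logic exists but is disconnected from the empty overlap events.
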(event `self.OverlapZone.OnComponentBeginOverlap`
  (params (OverlappedComponent :type "PrimitiveComponent Object Reference") (OtherActor :type "Actor Object Reference") (OtherComp :type "PrimitiveComponent Object Reference") (OtherBodyIndex :type Integer) (bFromSweep :type Boolean) (SweepResult :type "HitResult Structure (by ref)")))

(event `self.OverlapZone.OnComponentEndOverlap`
  (params (OverlappedComponent :type "PrimitiveComponent Object Reference") (OtherActor :type "Actor Object Reference") (OtherComp :type "PrimitiveComponent Object Reference") (OtherBodyIndex :type Integer)))

(event `/Game/Blueprints/BI_Interactable.OnPreInteract`)

(event `/Game/Blueprints/BI_Interactable.OnFinishInteract`)

(event `/Game/Blueprints/BI_Interactable.Interact`
  (`self.RPC_Server_openZone`))

(event `RPC_Server_openZone`
  (`self.Set Zone State` true)
  (bind _asbp_game_state (cast `/Game/Blueprints/NetworkingSetup/BP_GameState` (`GameplayStatics.GetGameState`)))
  (`self.RPC_openZone`)
  (`/Game/Blueprints/NetworkingSetup/BP_GameState.RPC_Server_ZoneOpened` _asbp_game_state null))

(event `RPC_openZone`
  (`self.Set Zone State` true))

(fn `CanInteract`
  (returns (CanInteract :type Boolean))
  (bind _asbp_game_state (cast `/Game/Blueprints/NetworkingSetup/BP_GameState` (`GameplayStatics.GetGameState`)))
  (return (>= (`/Game/Blueprints/NetworkingSetup/BP_GameState.Currency` _asbp_game_state) (`self.openPrice`))))

(fn `GetOpenState`
  (returns (OpenState :type Boolean))
  (return (`self.IsOpen`)))

(fn `Set Zone State`
  (params (NewOpenState :type Boolean))
  (bind _cube (`self.Cube`))
  (bind _output_get (set `self.IsOpen` NewOpenState))
  (`SceneComponent.SetHiddenInGame` _cube _output_get true)
  (if (`self.IsOpen`)
    (`PrimitiveComponent.SetCollisionProfileName` _cube "OverlapAll" true)
    (else
      (`PrimitiveComponent.SetCollisionProfileName` _cube "BlockAll" true))))

(fn `UserConstructionScript`)