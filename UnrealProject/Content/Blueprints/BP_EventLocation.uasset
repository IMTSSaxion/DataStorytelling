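; BP_EventLocation is a placeable marker Actor that spawns a puzzle Actor at its own transform.
; Spawn Puzzle gets the class from GetPuzzleType, which looks up the EventType variable in the PuzlleOptions map, and spawns it with collision adjusted but always spawning.
; An unmapped type only prints a red error, and no event in this Blueprint triggers the spawn itself.
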(fn `GetPuzzleType`
  (returns (PuzzleType :type "Actor Class Reference"))
  (locals (selectedPuzzleType :type "/Game/Blueprints/Puzzles/BP_PuzzleBase Class Reference"))
  (bind (_value _returnvalue) (`BlueprintMapLibrary.Map_Find` (`self.PuzlleOptions`) (`self.EventType`)))
  (set `local.selectedPuzzleType` _value)
  (if _returnvalue
    (return (`local.selectedPuzzleType`))
    (else
      (`KismetSystemLibrary.PrintString` "Unkown puzzle" true true (struct :`R` 0.8 :`A` 1.0)))))

(fn `Spawn Puzzle`
  (locals (NewLocalVar :type "Actor Class Reference" :default "/Script/Engine.BlueprintGeneratedClass'/Game/Blueprints/Puzzles/BP_PuzzleBase.BP_PuzzleBase_C'"))
  (bind _puzzletype (`self.GetPuzzleType`))
  (`|SpawnActorFromClass` _puzzletype (`self.GetTransform` self) "AdjustIfPossibleButAlwaysSpawn" "OverrideRootScale" null null))

(fn `UserConstructionScript`)