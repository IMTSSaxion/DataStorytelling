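; Gameplay game mode that alternates timed puzzle rounds with paused shop rounds, broadcasting phases, shop options and defeat through BP_GameState RPCs.
; Solved puzzles add shared currency, and puzzle spawns or solves recheck the active count to start or pause the defeat countdown.
; In the shop, a timer rotates a randomly chosen buyer until OpenZone unlocks a zone and resumes play.
; Shop cards are placeholders, and the win check is not wired up.
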(event `PuzzleStarted`
  (params (StartedPuzzle :type "/Game/Blueprints/Components/AC_Puzzle Object Reference"))
  (add `/Game/Blueprints/Components/AC_Puzzle.onResolve` StartedPuzzle (delegate `OnPuzzleSolved`)))

(event `OnPuzzleSolved`
  (`self.AddCurrency`)
  (bind _outactors (`GameplayStatics.GetAllActorsOfClass` "/Game/Blueprints/Puzzles/BP_PuzzleBase.BP_PuzzleBase_C" :!label _label))
  (bind _returnvalue (`KismetArrayLibrary.Array_Length` _outactors))
  (`KismetSystemLibrary.PrintString` (`KismetStringLibrary.Conv_IntToString` _returnvalue))
  (if (>= _returnvalue (`self.LoseNumber`))
    (if (`/Game/Blueprints/Components/AC_Timer.Paused` (`self.DefeatTimer`))
      (`/Game/Blueprints/Components/AC_Timer.Start` (`self.DefeatTimer`) (`self.LoseTime`) false))
    (else
      (`/Game/Blueprints/Components/AC_Timer.PauseTimer` (`self.DefeatTimer`)))))

(event `PuzzleSpawed`
  (goto _label))

(event `self.ReceiveTick`
  (params (DeltaSeconds :type "Float (single-precision)")))

(event `StartPlayRound`
  (`/Game/Blueprints/Components/AC_Timer.Start` (`self.RoundTimer`) (`self.RoundLength`) false)
  (`/Game/Blueprints/NetworkingSetup/BP_GameState.RPC_OnRoundStart` (`self.bpGameState`))
  (`/Game/Blueprints/NetworkingSetup/BP_GameState.SetPauseState` (`self.bpGameState`) false))

(event `StartShopRound`
  (bind _newparam (`self.CreateShopOptions`))
  (`/Game/Blueprints/NetworkingSetup/BP_GameState.RPC_OnRoundEnd` (`self.bpGameState`) _newparam)
  (`/Game/Blueprints/NetworkingSetup/BP_GameState.SetPauseState` (`self.bpGameState`) true)
  (`self.RestartShopTimer`)
  (`self.SelectShopBuyer`))

(event `self.ReceiveBeginPlay`
  (bind _asbp_game_state (cast `/Game/Blueprints/NetworkingSetup/BP_GameState` (`GameplayStatics.GetGameState`)))
  (bind _output_get (set `self.bpGameState` _asbp_game_state))
  (set `/Game/Blueprints/NetworkingSetup/BP_GameState.LoseTimer` (`self.LoseTime`) _output_get)
  ;[1 1 1] Round Timers Subscription
  (`self.StartPlayRound`)
  (add `/Game/Blueprints/Components/AC_Timer.On Finished` (`self.RoundTimer`) (delegate `HandleSpendTimer`))
  ;[1 1 1] Bind Shop Timers
  (add `/Game/Blueprints/Components/AC_Timer.On Finished` (`self.ShopTimer`) (delegate `HandleShopTimerFinished`))
  ;[1 1 1] Create Defeat Timer
  (add `/Game/Blueprints/Components/AC_Timer.On Finished` (`self.DefeatTimer`) (delegate `HandleDefeat`)))

(event `HandleSpendTimer`
  ;[1 1 1] Round Timers Subscription
  (`self.StartShopRound`))

(event `HandleShopTimerFinished`
  ;[1 1 1] Bind Shop Timers
  (`self.SelectShopBuyer`)
  (`/Game/Blueprints/Components/AC_Timer.RestartTimer` (`self.ShopTimer`)))

(event `HandleDefeat`
  ;[1 1 1] Create Defeat Timer
  (bind _asbp_game_state (cast `/Game/Blueprints/NetworkingSetup/BP_GameState` (`GameplayStatics.GetGameState`)))
  (`/Game/Blueprints/NetworkingSetup/BP_GameState.RPC_InvokeLose` _asbp_game_state)
  (`self.SetPauseState` true))

(event `SetPauseState`
  (params (`new PauseState` :type Boolean))
  (`/Game/Blueprints/NetworkingSetup/BP_GameState.SetPauseState` (`self.bpGameState`) `new PauseState`))

(event `OpenZone`
  (params (NewParam :type "PlayerController Object Reference"))
  (bind _outactors (`GameplayStatics.GetAllActorsOfClass` "/Game/Blueprints/BP_Zone.BP_Zone_C"))
  (for _array_element _outactors
    (if (not (`/Game/Blueprints/BP_Zone.IsOpen` _array_element))
      (`/Game/Blueprints/BP_Zone.RPC_Server_openZone` _array_element)
      (break)))
  (`self.StartPlayRound`))

(event `self.K2_PostLogin`
  (params (NewPlayer :type "PlayerController Object Reference"))
  (`KismetArrayLibrary.Array_AddUnique` (`/Game/Blueprints/NetworkingSetup/BP_GameState.PlayerStates` (`self.bpGameState`)) (`Controller.PlayerState` NewPlayer)))

(event `SelectShopBuyer`
  (bind _playerstates (`/Game/Blueprints/NetworkingSetup/BP_GameState.PlayerStates` (`self.bpGameState`)))
  (`/Game/Blueprints/NetworkingSetup/BP_GameState.RPC_PlayerSelected` (`self.bpGameState`) (`|GetArrayItem` _playerstates (`KismetMathLibrary.RandomInteger` (`KismetArrayLibrary.Array_Length` _playerstates)))))

(fn `AddCurrency`
  (bind _asbp_game_state (cast `/Game/Blueprints/NetworkingSetup/BP_GameState` (`GameplayStatics.GetGameState`)))
  (set `/Game/Blueprints/NetworkingSetup/BP_GameState.Currency` (+ (`/Game/Blueprints/NetworkingSetup/BP_GameState.Currency` _asbp_game_state) (`self.CurrencyPerPuzzle`)) _asbp_game_state))

(fn `CreateShopOptions`
  (returns (NewParam :type "Array of /Game/Blueprints/Data/ShopCard Structure"))
  (locals (CardOptions :type "Array of /Game/Blueprints/Data/ShopCard Structure"))
  (`KismetArrayLibrary.Array_Add` (`local.CardOptions`) (make `/Game/Blueprints/Data/ShopCard` 1 false "My First options" "/Game/Assets/Characters/Mannequins/Textures/Manny/T_Manny_02_N.T_Manny_02_N"))
  (`KismetArrayLibrary.Array_Add` (`local.CardOptions`) (make `/Game/Blueprints/Data/ShopCard` 100 false "My Second Options" "/Game/Assets/Cursor/T_Arrow.T_Arrow"))
  (return (`local.CardOptions`)))

(fn `GetCurrency`
  (returns (Value :type Integer))
  (return (`self.Currency`)))

(fn `HasWon`
  (returns (HasWon :type Boolean))
  (locals (NumberOfOpenedZones :type Integer) (hasWonBool :type Boolean :default false))
  (bind _numberofopenedzones (`local.NumberOfOpenedZones`))
  (for _array_element (`self.LevelZones`)
    (bind _openstate (`/Game/Blueprints/BI_Zone.GetOpenState` _array_element))
    (if _openstate
      (`/Engine/EditorBlueprintResources/StandardMacros.IncrementInt` _numberofopenedzones
        (:`  `
          (if (>= _numberofopenedzones (`self.VictoryNumber`))
            (return true))))))
  (return false))

(fn `LoseActions`
  (`GameplayStatics.SetGamePaused` true))

(fn `RestartShopTimer`
  (`/Game/Blueprints/Components/AC_Timer.Start` (`self.ShopTimer`) (`self.ShopLength`) true))

(fn `UserConstructionScript`
  (bind _outactors (`GameplayStatics.GetAllActorsWithInterface` "/Game/Blueprints/BI_Zone.BI_Zone_C"))
  (for _array_element _outactors
    (bind _asbi_zone (cast `/Game/Blueprints/BI_Zone` _array_element))
    (`KismetArrayLibrary.Array_Add` (`self.LevelZones`) _asbi_zone)))

(fn `WinActions`
  (`KismetSystemLibrary.PrintString` "We won?"))