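; AC_SHOP is a shop component that randomly picks which player is the current buyer.
; It caches BP_GameState on BeginPlay for later use.
; SelectShopBuyer tries to avoid LastVoter by stepping an index, but each random index is drawn separately, so that player can still be chosen.
; The result is stored as CurrentPlayer, passed to CallOnBuyingPlayerChanged and sent to the game state through RPCPlayerSelected.
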(event `self.ReceiveBeginPlay`
  (bind _asbp_game_state (cast `/Game/Blueprints/NetworkingSetup/BP_GameState` (`GameplayStatics.GetGameState`)))
  (set `self.GameState` _asbp_game_state))

(event `SelectShopBuyer`
  (bind _players (`self.Players`))
  (bind _currentplayer (`self.CurrentPlayer`))
  (bind _returnvalue (`KismetArrayLibrary.Array_Length` _players))
  (bind _returnvalue_2 (`KismetMathLibrary.RandomInteger` _returnvalue))
  (bind _output (`|GetArrayItem` _players _returnvalue_2))
  (if (!= _output (`self.LastVoter`))
    (set `self.CurrentPlayer` _output)
    (else
      (set `self.CurrentPlayer` (`|GetArrayItem` _players (mod (+ _returnvalue_2 1) _returnvalue)))))
  (`self.OnBuyingPlayerChanged` _currentplayer)
  (`/Game/Blueprints/NetworkingSetup/BP_GameState.RPC_PlayerSelected` (`self.GameState`) _currentplayer))