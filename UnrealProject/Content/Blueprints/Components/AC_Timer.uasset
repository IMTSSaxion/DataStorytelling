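; AC_Timer is a reusable countdown timer component that fires an OnFinished callback when its time runs out.
; Start sets the length and an ignore-pause flag, and RestartTimer resets the countdown to that length.
; Tick counts down only while BP_GameState is not paused, unless the timer ignores pause.
; GetProgress returns the remaining fraction of the timer, falling from one toward zero.
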(event `self.ReceiveBeginPlay`
  (bind _asbp_game_state (cast `/Game/Blueprints/NetworkingSetup/BP_GameState` (`GameplayStatics.GetGameState`)))
  (set `self.GameState` _asbp_game_state))

(event `Start`
  (params (Time :type "Float (double-precision)") (IgnorePause :type Boolean))
  (set `self.TimerLength` Time)
  (set `self.Timer` Time)
  (set `self.Ignore Pause` IgnorePause))

(event `RestartTimer`
  (set `self.Timer` (`self.TimerLength`)))

(event `self.ReceiveTick`
  (params (DeltaSeconds :type "Float (single-precision)"))
  (if (or (`self.Ignore Pause`) (not (`/Game/Blueprints/NetworkingSetup/BP_GameState.IsGamePaused` (`self.GameState`))))
    (if (> (`self.Timer`) 0.0)
      (bind _output_get (set `self.Timer` (- (`self.Timer`) DeltaSeconds)))
      (if (<= _output_get 0.0)
        (`self.On Finished`)))))

(fn `GetProgress`
  (returns (Progress :type "Float (double-precision)"))
  (return (/ (`self.Timer`) (`self.TimerLength`))))