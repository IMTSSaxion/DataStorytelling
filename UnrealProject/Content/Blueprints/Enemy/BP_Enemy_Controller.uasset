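; BP_Enemy_Controller is the AI controller for enemies, running their behavior tree and honoring the game's pause state.
; On BeginPlay it runs BT_Enemy, caches the BP_GameState and binds to its OnPauseStateChanged event.
; The handler stops the brain component's logic on pause and starts it again on unpause.
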(event `self.ReceiveBeginPlay`
  (`self.RunBehaviorTree` "/Game/Blueprints/Enemy/BT_Enemy.BT_Enemy")
  (bind _asbp_game_state (cast `/Game/Blueprints/NetworkingSetup/BP_GameState` (`GameplayStatics.GetGameState`)))
  (bind _output_get (set `self.GameState` _asbp_game_state))
  (add `/Game/Blueprints/NetworkingSetup/BP_GameState.OnPauseStateChanged` _output_get (delegate `HandlePauseChange`)))

(event `HandlePauseChange`
  (params (pauseState :type Boolean))
  (bind _braincomponent (`AIController.BrainComponent` (`AIBlueprintHelperLibrary.GetAIController` self)))
  (if pauseState
    (`BrainComponent.StopLogic` _braincomponent "")
    (else
      (`BrainComponent.StartLogic` _braincomponent))))

(fn `UserConstructionScript`)