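; Function library that gathers the event-interactable actors in the level whose active state matches a requested puzzle state.
; CanEventWithState fetches every actor implementing BI_EventInteractable, passes the array through CastArray, and keeps entries whose IsActive equals the requested value.
; CastArray is meant to convert actors to interface references, but its cast-and-add logic is disconnected from its empty loop, so it never fills its result.
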(fn `CanEventWithState`
  (params (Active :type Boolean))
  (returns (FillteredArray :type "Array of /Game/Blueprints/Puzzles/BI_EventInteractable Interface"))
  (locals (ActiveEvents :type "Array of /Game/Blueprints/Puzzles/BI_EventInteractable Interface") (RequestedPuzzleState :type Boolean))
  (set `local.RequestedPuzzleState` Active)
  (bind _outactors (`GameplayStatics.GetAllActorsWithInterface` null "/Game/Blueprints/Puzzles/BI_EventInteractable.BI_EventInteractable_C"))
  (bind _castedarray (`self.CastArray` _outactors))
  (for _array_element _castedarray
    (bind _isactive (`/Game/Blueprints/Puzzles/BI_EventInteractable.IsActive` _array_element))
    (if (== _isactive (`local.RequestedPuzzleState`))
      (`KismetArrayLibrary.Array_Add` (`local.ActiveEvents`) _array_element)))
  (return (`local.ActiveEvents`)))

(fn `CastArray`
  (params (Array :type "Array of Actor Object Reference"))
  (returns (CastedArray :type "Array of /Game/Blueprints/Puzzles/BI_EventInteractable Interface"))
  (locals (IntermidiateArray :type "Array of /Game/Blueprints/Puzzles/BI_EventInteractable Interface"))
  (for _ Array
    _))