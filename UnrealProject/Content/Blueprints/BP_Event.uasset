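; BP_Event is a world trigger actor that starts a puzzle when a character overlaps its Cube.
; Overlaps from actors implementing BI_character spawn a BP_PuzzleBase at the trigger's transform, unless a previously created puzzle is still valid.
; It binds a kill handler to the puzzle component's OnResolve and calls InitMessage.
; A kill event destroys the trigger actor.
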(event `self.Cube.OnComponentBeginOverlap`
  (params (OverlappedComponent :type "PrimitiveComponent Object Reference") (OtherActor :type "Actor Object Reference") (OtherComp :type "PrimitiveComponent Object Reference") (OtherBodyIndex :type Integer) (bFromSweep :type Boolean) (SweepResult :type "HitResult Structure (by ref)"))
  (if (`KismetSystemLibrary.DoesImplementInterface` OtherActor "/Game/Blueprints/BI_character.BI_character_C")
    (`self.IsPuzzleActive`
      (:`IsNotActivated`
        (bind _returnvalue (`|SpawnActorFromClass` "/Game/Blueprints/BP_PuzzleBase.BP_PuzzleBase_C" (`self.GetTransform`) "AlwaysSpawn" "OverrideRootScale" null null))
        (bind _output_get (set `self.PuzzleCreated` _returnvalue))
        (bind _ac_puzzle (`/Game/Blueprints/BP_PuzzleBase.AC_Puzzle` _output_get))
        (add `/Game/Blueprints/Components/AC_Puzzle.onResolve` _ac_puzzle (delegate `On Event Killed`))
        (message `/Game/Blueprints/BI_puzzle.Init` _ac_puzzle)))))

(event `On Event Killed`
  (`self.K2_DestroyActor`))

(fn `UserConstructionScript`)