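; Game state Blueprint that relays round, shop, pause and win/lose state between BP_GameplayGameMode and listeners.
; RPC events fire notifications for round start and end, shopper changes, win and loss, storing new shop options at round end.
; Tick calls a server RPC that copies round progress and shop timer from the game mode.
; Zone opening forwards to the game mode, and a zone-opened RPC checks HasWon to trigger victory.
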(event `self.ReceiveBeginPlay`
  (bind _asbp_gameplay_game_mode (cast `/Game/Blueprints/GameModes/BP_GameplayGameMode` (`GameplayStatics.GetGameMode`)))
  (set `self.GameMode` _asbp_gameplay_game_mode))

(event `RPC_PlayerSelected`
  (params (NewVoter :type "PlayerState Object Reference"))
  (`/Engine/EditorBlueprintResources/StandardMacros.IsValid` NewVoter
    (:`Is Valid`
      (`self.OnShoperChanged` NewVoter))))

(event `RPC_InvokeLose`
  (`self.OnLose`))

(event `RPC_InvokeWin`
  (`self.OnWin`))

(event `RPC_OnRoundEnd`
  (params (ShopOptions :type "Array of /Game/Blueprints/Data/ShopCard Structure"))
  (set `self.NewShopOptions` ShopOptions)
  (`self.OnRoundEnd`))

(event `RPC_OnRoundStart`
  (`self.OnRoundStart`))

(event `RPC_Server_ZoneOpened`
  (params (playerController :type "PlayerController Object Reference"))
  (bind _asbp_gameplay_game_mode (cast `/Game/Blueprints/GameModes/BP_GameplayGameMode` (`GameplayStatics.GetGameMode`)))
  (bind _haswon (`/Game/Blueprints/GameModes/BP_GameplayGameMode.HasWon` _asbp_gameplay_game_mode))
  (if _haswon
    (`self.RPC_InvokeWin`)))

(event `self.ReceiveTick`
  (params (DeltaSeconds :type "Float (single-precision)"))
  (`self.RPC_Server_GetLatestTimer`))

(event `RPC_Server_GetLatestTimer`
  (bind _progress (`/Game/Blueprints/Components/AC_Timer.GetProgress` (`/Game/Blueprints/GameModes/BP_GameplayGameMode.RoundTimer` (`self.GameMode`))))
  (set `self.RoundProgressBar` _progress)
  (set `self.ShopTimer` (`/Game/Blueprints/Components/AC_Timer.Timer` (`/Game/Blueprints/GameModes/BP_GameplayGameMode.ShopTimer` (`self.GameMode`)))))

(event `SetPauseState`
  (params (newPauseState :type Boolean))
  (bind _output_get (set `self.IsGamePaused` newPauseState))
  (`self.OnPauseStateChanged` _output_get))

(event `/Game/Blueprints/Interfaces/BI_ZonesControls.OpenZone`
  (`self.RPC_Server_OpenZone`))

(event `RPC_Server_OpenZone`
  (`/Game/Blueprints/GameModes/BP_GameplayGameMode.OpenZone` (`self.GameMode`) null))

(fn `GetPlayersData`
  (returns (PlayerArray :type "Array of PlayerState Object Reference"))
  (locals (Players :type "Array of PlayerState Object Reference"))
  (for _array_element (`self.PlayerArray`)
    (`KismetArrayLibrary.Array_Add` (`local.Players`) _array_element)
    (return (`local.Players`)))
  (return (`local.Players`)))

(fn `OnRep_Test`
  (`KismetSystemLibrary.PrintString` "Rep notify"))

(fn `UserConstructionScript`)